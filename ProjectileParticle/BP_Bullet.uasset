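; BP_Bullet is a projectile that adds knockback to the Ba_Type actor it hits, ignoring its own Player.
; It spawns an attached BP_MissileTrail and removes it on EndPlay.
; Each tick, the game mode's WindOrigin pushes its velocity radially outward by WindPower.
; On overlap, impact speed is added to the target's KnockBack, with the total doubled during Player's arrow power-up, then the bullet destroys itself.
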(event OnComponentBeginOverlap(StaticMesh)
  (params (OverlappedComponent :type Primitive%20Component%20Object%20Reference) (OtherActor :type Actor%20Object%20Reference) (OtherComp :type Primitive%20Component%20Object%20Reference) (OtherBodyIndex :type Integer) (bFromSweep :type Boolean) (SweepResult :type Hit%20Result%20Structure%20%28by%20ref%29))
  (bind _player (Variables|Default|GetPlayer))
  (Utilities|IsValid (Variables|Default|GetPlayer)
    (:Is%20Valid
      _)
    (:Is%20Not%20Valid
      (Utilities|FlowControl|Delay 0.05)))
  (bind _asba_type (Utilities|Casting|CastToBa_Type OtherActor))
  (if (not (== _asba_type _player))
    (if (> (Variables|/Game/Characters/Balance/Ba_Type.Ba_Type_C|GetArrowPowerUpTime (.AsBa%20Type (Utilities|Casting|CastToBa_Type _player))) 0.0)
      (Variables|/Game/Characters/Balance/Ba_Type.Ba_Type_C|SetKnockBack _asba_type (* (+ (Variables|/Game/Characters/Balance/Ba_Type.Ba_Type_C|GetKnockBack _asba_type) (Math|Vector|VectorLength (Transformation|GetVelocity))) 2.0))
      (Actor|DestroyActor)
      (else
        (Variables|/Game/Characters/Balance/Ba_Type.Ba_Type_C|SetKnockBack _asba_type (+ (Variables|/Game/Characters/Balance/Ba_Type.Ba_Type_C|GetKnockBack _asba_type) (Math|Vector|VectorLength (Transformation|GetVelocity))))
        (Actor|DestroyActor)))))

(event EventBeginPlay
  (bind _asba_mode (Utilities|Casting|CastToBa_Mode (Game|GetGameMode)))
  (Variables|Default|SetWindOrigin (Variables|/Game/Characters/Balance/Ba_Mode.Ba_Mode_C|GetWindOrigin _asba_mode))
  (bind _returnvalue (Game|SpawnActorfromClass "/Game/MissileTrailParticle/Blueprints/BP_MissileTrail.BP_MissileTrail_C" (Transformation|GetActorTransform) "Undefined" 0 0))
  (bind _output_get (Variables|Default|SetTrailActor _returnvalue))
  (Class|Actor|AttachRootComponentto _output_get (Variables|Default|GetStaticMesh) "None" "SnapToTarget" true))

(event Collision|EventActorBeginOverlap
  (params (OtherActor :type Actor%20Object%20Reference)))

(event EventTick
  (params (DeltaSeconds :type Float%20%28single-precision%29))
  (bind _windorigin (Variables|Default|GetWindOrigin))
  (bind _projectilemovement (Variables|Default|GetProjectileMovement))
  (Utilities|IsValid _windorigin
    (:Is%20Valid
      (Variables|/Script/Engine.MovementComponent|SetVelocity _projectilemovement (+ (Variables|/Script/Engine.MovementComponent|GetVelocity _projectilemovement) (* (Math|Vector|Normalize (- (Transformation|GetActorLocation) (Transformation|GetActorLocation _windorigin))) (Variables|/Game/BP_WindOrigin.BP_WindOrigin_C|GetWindPower _windorigin)))))))

(event EventEndPlay
  (params (EndPlayReason :type EEndPlayReason%20Enum :default "Destroyed"))
  (Actor|DestroyActor (Variables|Default|GetTrailActor)))

(fn ConstructionScript)