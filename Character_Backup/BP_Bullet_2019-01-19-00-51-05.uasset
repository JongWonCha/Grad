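; BP_Bullet is a projectile actor whose flight is pushed by wind from a WindOrigin actor.
; Every Tick it adds a unit vector pointing from WindOrigin toward the bullet to its ProjectileMovement velocity, steadily accelerating it away from that origin.
; The push is not scaled by delta time, so its strength depends on frame rate.
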(event EventBeginPlay)

(event Collision|EventActorBeginOverlap
  (params (OtherActor :type Actor%20Object%20Reference)))

(event EventTick
  (params (DeltaSeconds :type Float%20%28single-precision%29))
  (bind _projectilemovement (Variables|Default|GetProjectileMovement))
  (bind _output_get (Variables|/Script/Engine.MovementComponent|SetVelocity _projectilemovement (+ (Variables|/Script/Engine.MovementComponent|GetVelocity _projectilemovement) (Math|Vector|Normalize (- (Transformation|GetActorLocation) (Transformation|GetActorLocation (Variables|Default|GetWindOrigin))))))))

(fn ConstructionScript)